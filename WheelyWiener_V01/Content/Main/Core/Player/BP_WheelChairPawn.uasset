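; Player pawn for a wheelchair character, with enhanced input for movement, mouse look and a horn sound.
; Movement input feeds the BPCWheelMovement component, while physical animation simulates the skeletal mesh bodies below a named bone.
; Microphone envelope from AudioCapture goes through an RPC, where thresholds and a hold timer set a speaking state that smoothly interpolates a jaw-open amount for lip movement.
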(event `self.ReceiveTick`
  (params (DeltaSeconds :type "Float (single-precision)"))
  (set `self.Delta Time X` DeltaSeconds))

(event `self.ReceiveBeginPlay`
  (bind _physicalanimation (`self.PhysicalAnimation`))
  (bind _body_name (`self.Body Name`))
  (bind _asbp_wwcontroller (cast `/Game/Main/Core/Framework/BP_WWController` (`self.GetController`)))
  (bind _output_get (set `self.PlayerControllerReference` _asbp_wwcontroller))
  (`EnhancedInputSubsystemInterface.AddMappingContext` (pcsubsystem `EnhancedInputLocalPlayerSubsystem` _output_get) "/Game/Main/Core/Inputs/IMC_Inputs.IMC_Inputs" 0 (struct))
  (`PhysicalAnimationComponent.SetSkeletalMeshComponent` _physicalanimation (`self.SkeletalMesh`))
  (`PhysicalAnimationComponent.ApplyPhysicalAnimationSettingsBelow` _physicalanimation _body_name (make `PhysicalAnimationData` true 50.0 50.0 50.0 50.0) true)
  (`SkeletalMeshComponent.SetAllBodiesBelowSimulatePhysics` (`self.SkeletalMesh`) _body_name true false))

(event `EnhancedInput|/Game/Main/Core/Inputs/Actions/IA_ForwardBackward`
  (params (ActionValue :type "Float (double-precision)") (ElapsedSeconds :type "Float (double-precision)") (TriggeredSeconds :type "Float (double-precision)") (InputAction :type "InputAction Object Reference" :default "/Game/Main/Core/Inputs/Actions/IA_ForwardBackward.IA_ForwardBackward"))
  (bind _bpc_wheelmovement (`self.BPC_WheelMovement`))
  (:`Triggered`
    (set `/Game/Main/Core/Components/BPC_WheelMovement.InputForward` ActionValue _bpc_wheelmovement))
  (:`Completed`
    (set `/Game/Main/Core/Components/BPC_WheelMovement.InputForward` 0.0 _bpc_wheelmovement)))

(event `EnhancedInput|/Game/Main/Core/Inputs/Actions/IA_LeftRight`
  (params (ActionValue :type "Float (double-precision)") (ElapsedSeconds :type "Float (double-precision)") (TriggeredSeconds :type "Float (double-precision)") (InputAction :type "InputAction Object Reference" :default "/Game/Main/Core/Inputs/Actions/IA_LeftRight.IA_LeftRight"))
  (bind _bpc_wheelmovement (`self.BPC_WheelMovement`))
  (:`Triggered`
    (set `/Game/Main/Core/Components/BPC_WheelMovement.InputRight` ActionValue _bpc_wheelmovement))
  (:`Completed`
    (set `/Game/Main/Core/Components/BPC_WheelMovement.InputRight` 0.0 _bpc_wheelmovement)))

(event `EnhancedInput|/Game/Main/Core/Inputs/Actions/IA_Horn`
  (params (ActionValue :type Boolean) (ElapsedSeconds :type "Float (double-precision)") (TriggeredSeconds :type "Float (double-precision)") (InputAction :type "InputAction Object Reference" :default "/Game/Main/Core/Inputs/Actions/IA_Horn.IA_Horn"))
  (:`Started`
    (`GameplayStatics.PlaySoundAtLocation` "/Game/Main/Sounds/Player/SW_Horn_00.SW_Horn_00" (`self.K2_GetActorLocation`) (struct) 1.0 1.0 0.0 null null null null)))

(event `EnhancedInput|/Game/Main/Core/Inputs/Actions/IA_Look`
  (params (ActionValue :type "Vector2D Structure") (ElapsedSeconds :type "Float (double-precision)") (TriggeredSeconds :type "Float (double-precision)") (InputAction :type "InputAction Object Reference" :default "/Game/Main/Core/Inputs/Actions/IA_Look.IA_Look"))
  (bind (_x _y) (`KismetMathLibrary.BreakVector2D` ActionValue))
  (:`Triggered`
    (`self.AddControllerYawInput` _x)
    (`self.AddControllerPitchInput` _y)))

(event `self.AudioCapture.OnAudioEnvelopeValue`
  (params (EnvelopeValue :type "Float (single-precision)"))
  ; Capture Audio
  (set `self.Envelope Value` EnvelopeValue)
  (bind _output_get (set `self.RawMicVolume` (`KismetMathLibrary.MapRangeClamped` (`self.Envelope Value`) 0.005 0.1 0.0 1.0)))
  (`self.RPC_LocalMic` _output_get))

(event `RPC_LocalMic`
  (params (RawMic :type "Float (double-precision)"))
  ; Lip Movement on Server
  (`|ExecutionSequence`
    (:`then_0`
      (if (> RawMic (`self.ThresholdOn`))
        (set `self.SpeakingTimer` (`self.SpeakingHoldTime`))
        (set `self.IsSpeaking` true)
        (elif (< RawMic (`self.ThresholdOff`))
          (set `self.SpeakingTimer` (- (`self.SpeakingTimer`) (`self.Delta Time X`)))
          (if (<= (`self.SpeakingTimer`) 0.0)
            (set `self.IsSpeaking` false)
            (set `self.SpeakingTimer` 0.0)))))
    (:`then_1`
      (set `self.JawOpenAmount` (`KismetMathLibrary.FInterpTo` (`self.JawOpenAmount`) (`KismetMathLibrary.SelectFloat` (`self.OpenAmount`) 0.0 (`self.IsSpeaking`)) (`self.Delta Time X`) (`KismetMathLibrary.SelectFloat` (`self.OpenSpeed`) (`self.CloseSpeed`) (`self.IsSpeaking`)))))))

(fn `UserConstructionScript`)