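; BP_GrabPistol is a held item that carries physics objects through its owning character's PhysicsHandle; starting a grab happens outside this file.
; While the locally controlled owner is grabbing, Tick updates the handle or releases it if the component is invalid or stops simulating physics.
; UpdateHeldObject holds the target along the eye view at a clamped, mouse-wheel-adjusted distance plus height offset, drawing the beam as a debug line.
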(event `self.ReceiveBeginPlay`
  (`parent.ReceiveBeginPlay`))

(event `self.ReceiveActorBeginOverlap`
  (params (OtherActor :type "Actor Object Reference"))
  (`parent.ReceiveActorBeginOverlap` OtherActor))

(event `self.ReceiveTick`
  (params (DeltaSeconds :type "Float (single-precision)"))
  (bind _asbp_character_master (cast `/Game/Main/Core/Player/BP_CharacterMaster` (`self.GetOwner`)))
  (if (and (`/Game/Main/Core/Player/BP_CharacterMaster.bGrabbing` _asbp_character_master) (`Pawn.IsLocallyControlled` _asbp_character_master))
    (bind _physicshandle (`/Game/Main/Core/Player/BP_CharacterMaster.PhysicsHandle` _asbp_character_master))
    (bind _returnvalue (`PhysicsHandleComponent.GetGrabbedComponent` _physicshandle))
    (`/Engine/EditorBlueprintResources/StandardMacros.IsValid` _returnvalue
      (:`Is Valid`
        (if (`SceneComponent.IsSimulatingPhysics` _returnvalue "None")
          (`self.UpdateHeldObject` _returnvalue _asbp_character_master)
          (else
            (`PhysicsHandleComponent.ReleaseComponent` _physicshandle)
            (set `/Game/Main/Core/Player/BP_CharacterMaster.bGrabbing` false _asbp_character_master))))
      (:`Is Not Valid`
        (`PhysicsHandleComponent.ReleaseComponent` _physicshandle)
        (set `/Game/Main/Core/Player/BP_CharacterMaster.bGrabbing` false _asbp_character_master)))))

(fn `UpdateHeldObject`
  (params (GrabbedComponent :type "PrimitiveComponent Object Reference") (Character :type "/Game/Main/Core/Player/BP_CharacterMaster Object Reference"))
  (bind (_outlocation _outrotation) (`self.GetActorEyesViewPoint` Character))
  (set `self.GrabDistance` (`KismetMathLibrary.FClamp` (+ (`self.GrabDistance`) (* (`PlayerController.GetInputAnalogKeyState` (`/Game/Main/Core/Player/BP_CharacterMaster.PlayerControllerReference` Character) "MouseWheelAxis") (`self.GrabDistanceStep`))) (`self.MinGrabDistance`) (`self.MaxGrabDistance`)))
  (`PhysicsHandleComponent.SetTargetLocation` (`/Game/Main/Core/Player/BP_CharacterMaster.PhysicsHandle` Character) (+ (+ _outlocation (* (`KismetMathLibrary.GetForwardVector` _outrotation) (`self.GrabDistance`))) (`KismetMathLibrary.MakeVector` 0.0 0.0 (`self.GrabHeightOffset`))))
  (`KismetSystemLibrary.DrawDebugLine` (`SceneComponent.K2_GetComponentLocation` (`self.StaticMesh`)) (`SceneComponent.K2_GetComponentLocation` GrabbedComponent) (struct :`G` 1.0 :`B` 0.4 :`A` 1.0) 0.0 3.0))

(fn `UserConstructionScript`
  (`parent.UserConstructionScript`))