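; Sauce splat hazard that flags characters' wheelchair movement while they are inside its sphere.
; On BeginPlay the server picks a random splat index and sets a timed lifespan, and a dynamic decal material takes that index as its variant.
; Server-only sphere begin and end overlaps set and clear OnSplat on the BP_CharacterMaster's wheelchair movement component.
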(event `self.ReceiveBeginPlay`
  (bind _decal (`self.Decal`))
  (if (`self.HasAuthority`)
    (set `self.SplatIndex` (`KismetMathLibrary.RandomIntegerInRange` 0 3))
    (`self.SetLifeSpan` 60.0))
  (bind _returnvalue (`DecalComponent.CreateDynamicMaterialInstance` _decal))
  (`DecalComponent.SetDecalMaterial` _decal _returnvalue)
  (`MaterialInstanceDynamic.SetScalarParameterValue` _returnvalue "Index" (`KismetMathLibrary.Conv_IntToDouble` (`self.SplatIndex`))))

(event `self.Sphere.OnComponentBeginOverlap`
  (params (OverlappedComponent :type "PrimitiveComponent Object Reference") (OtherActor :type "Actor Object Reference") (OtherComp :type "PrimitiveComponent Object Reference") (OtherBodyIndex :type Integer) (bFromSweep :type Boolean) (SweepResult :type "HitResult Structure (by ref)"))
  (if (`self.HasAuthority`)
    (bind _asbp_character_master (cast `/Game/Main/Core/Player/BP_CharacterMaster` OtherActor))
    (set `/Game/Main/Core/Components/BPC_WheelchairMovement.bOnSplat` true (`/Game/Main/Core/Player/BP_CharacterMaster.BPC_WheelchairMovement` _asbp_character_master))))

(event `self.Sphere.OnComponentEndOverlap`
  (params (OverlappedComponent :type "PrimitiveComponent Object Reference") (OtherActor :type "Actor Object Reference") (OtherComp :type "PrimitiveComponent Object Reference") (OtherBodyIndex :type Integer))
  (if (`self.HasAuthority`)
    (bind _asbp_character_master (cast `/Game/Main/Core/Player/BP_CharacterMaster` OtherActor))
    (set `/Game/Main/Core/Components/BPC_WheelchairMovement.bOnSplat` false (`/Game/Main/Core/Player/BP_CharacterMaster.BPC_WheelchairMovement` _asbp_character_master))))

(fn `UserConstructionScript`)