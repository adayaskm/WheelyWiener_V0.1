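; Actor component that drives physics-based wheelchair movement on the owning BP_CharacterMaster's capsule.
; Movement ground-traces via CheckIfFalling, applies a downward impulse while airborne, and swaps damping on splat surfaces.
; In the Normal state it calls a server RPC that applies forward force with sprint scaling and yaw torque, then clamps speed.
; A separate Jump function applies an upward impulse, gated on IsFalling, which is true when the trace hits ground.
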(event `self.ReceiveBeginPlay`
  (bind _asbp_character_master (cast `/Game/Main/Core/Player/BP_CharacterMaster` (`self.GetOwner`)))
  (set `self.PlayerReference` _asbp_character_master))

(event `Movement`
  (bind _normalfriction (`self.NormalFriction`))
  (bind _splatfriction (`self.SplatFriction`))
  (bind _capsule (`/Game/Main/Core/Player/BP_CharacterMaster.Capsule` (`self.PlayerReference`)))
  (bind _capsule_2 (`/Game/Main/Core/Player/BP_CharacterMaster.Capsule` (`self.PlayerReference`)))
  ; Movement Setup
  (`self.CheckIfFalling`)
  (if (`self.bIsJump`)
    (`PrimitiveComponent.AddImpulse` _capsule (* (`SceneComponent.GetUpVector` _capsule) -1.0 10000.0) "None" false))
  (if (`self.bOnSplat`)
    (`PrimitiveComponent.SetLinearDamping` _capsule_2 _splatfriction)
    (`PrimitiveComponent.SetAngularDamping` _capsule_2 _splatfriction)
    (else
      (`PrimitiveComponent.SetLinearDamping` _capsule_2 _normalfriction)
      (`PrimitiveComponent.SetAngularDamping` _capsule_2 _normalfriction)))
  (switch `/Game/Main/Core/Enums/E_WheelchairState` (`self.CurrentState`)
    (:`NewEnumerator0`
      (`self.ServerRPC_Movement`))))

(event `ServerRPC_Movement`
  (bind _maxspeed (`self.MaxSpeed`))
  (bind _capsule (`/Game/Main/Core/Player/BP_CharacterMaster.Capsule` (`self.PlayerReference`)))
  ; Server RPC Movement
  (`PrimitiveComponent.AddForce` _capsule (* (`SceneComponent.GetForwardVector` (`/Game/Main/Core/Player/BP_CharacterMaster.Capsule` (`self.PlayerReference`))) (* (`self.ForwardInput`) (`self.ForwardForce`) (`self.SprintMultiplier`))) "None" false)
  (`PrimitiveComponent.AddTorqueInRadians` _capsule (`KismetMathLibrary.MakeVector` 0.0 0.0 (* (`self.TurnInput`) (`self.TurnTorque`))) "None" false)
  (bind _returnvalue (`PrimitiveComponent.GetPhysicsLinearVelocity` _capsule "None"))
  (if (> (`KismetMathLibrary.VSize` _returnvalue) _maxspeed)
    (`PrimitiveComponent.SetPhysicsLinearVelocity` _capsule (* (`KismetMathLibrary.Normal` _returnvalue) _maxspeed) false "None")))

(fn `CheckIfFalling`
  (returns (`Success?` :type Boolean))
  (bind _capsule (`/Game/Main/Core/Player/BP_CharacterMaster.Capsule` (`self.PlayerReference`)))
  (bind _returnvalue (`SceneComponent.K2_GetComponentLocation` _capsule))
  (bind _outhit (`KismetSystemLibrary.LineTraceSingle` _returnvalue (+ _returnvalue (* (`SceneComponent.GetUpVector` _capsule) -1.0 100.0)) "TraceTypeQuery1" false (`|MakeArray` (`self.PlayerReference`) :!type "Actor Object Reference") "ForOneFrame"))
  (bind _output_get (set `self.bIsFalling` (`GameplayStatics.BreakHitResult` _outhit)))
  (set `self.bIsJump` (== _output_get false))
  (return _output_get))

(fn `Jump`
  (params (bIsJump :type Boolean))
  (bind _capsule (`/Game/Main/Core/Player/BP_CharacterMaster.Capsule` (`self.PlayerReference`)))
  (`self.bIsFalling`
    (:`then`
      (`PrimitiveComponent.AddImpulse` _capsule (* (`SceneComponent.GetUpVector` _capsule) 100000.0) "None" false)
      (set `self.bIsJump` bIsJump))
    (:`else`)))