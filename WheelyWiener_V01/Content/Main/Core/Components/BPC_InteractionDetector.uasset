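; Player component that handles picking up, holding and dropping BP_ItemMaster items.
; InteractDetect sphere-traces from the camera, drops any held item, then attaches the item it hit.
; Attaching disables the item's physics and collision, snaps it to a socket on the character mesh and grants its ShotAbility through the ability system.
; Detaching restores physics and collision and applies a mostly upward impulse, without removing the granted ability.
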(event `self.ReceiveBeginPlay`
  (bind _asbp_character_master (cast `/Game/Main/Core/Player/BP_CharacterMaster` (`self.GetOwner`)))
  (bind _output_get (set `self.PlayerReference` _asbp_character_master))
  (bind _asbp_wwcontroller (cast `/Game/Main/Core/Framework/BP_WWController` (`Pawn.GetController` _output_get)))
  (set `self.As BP WWController` _asbp_wwcontroller))

(event `InteractDetect`
  (bind _playercameramanager (`PlayerController.PlayerCameraManager` (`self.As BP WWController`)))
  (bind _returnvalue (`SceneComponent.K2_GetComponentLocation` (`Actor.RootComponent` _playercameramanager)))
  ; Interact Trace
  (bind _outhit (`KismetSystemLibrary.SphereTraceSingle` _returnvalue (+ _returnvalue (* (`SceneComponent.GetForwardVector` (`Actor.RootComponent` _playercameramanager)) 1200.0)) 25.0 "TraceTypeQuery3" false (`|MakeArray` (`self.PlayerReference`) (`self.HeldItem`) :!type "Actor Object Reference") "ForOneFrame"))
  (`self.HeldItem`
    (:`then`
      (`self.DetachItem` (`self.HeldItem`))
      (bind (_bblockinghit _binitialoverlap _time _distance _location _impactpoint _normal _impactnormal _physmat _hitactor) (`GameplayStatics.BreakHitResult` _outhit))
      (`self.AttachItem` _hitactor))
    (:`else`
      (`self.AttachItem` _hitactor))))

(fn `AttachItem`
  (params (Actor :type "Actor Object Reference"))
  (bind _playerreference (`self.PlayerReference`))
  (bind _helditem (`self.HeldItem`))
  (bind _staticmesh (`/Game/Main/Core/Items/BP_ItemMaster.StaticMesh` _helditem))
  (bind _asbp_item_master (cast `/Game/Main/Core/Items/BP_ItemMaster` Actor))
  (bind _output_get (set `self.HeldItem` _asbp_item_master))
  (`Actor.SetOwner` _output_get _playerreference)
  (bind _iteminforeference (`/Game/Main/Core/Items/BP_ItemMaster.ItemInfoReference` _asbp_item_master))
  (bind _output_get_2 (set `self.EquippedItemInfo` _iteminforeference))
  (bind _shotability (`/Game/Main/Core/DataAssets/PDA_ItemInfo.ShotAbility` _iteminforeference))
  (if (`KismetSystemLibrary.IsValidClass` _shotability)
    (`AbilitySystemComponent.K2_GiveAbility` (`/Game/Main/Core/Player/BP_CharacterMaster.AbilitySystem` _playerreference) _shotability 0 -1))
  (`PrimitiveComponent.SetSimulatePhysics` _staticmesh false)
  (`SceneComponent.K2_SetRelativeLocationAndRotation` :`self` _staticmesh)
  (`PrimitiveComponent.SetCollisionEnabled` _staticmesh "NoCollision")
  (`PrimitiveComponent.SetCollisionEnabled` (`/Game/Main/Core/Items/BP_ItemMaster.Sphere` _helditem) "NoCollision")
  (`Actor.K2_AttachToComponent` _helditem (`/Game/Main/Core/Player/BP_CharacterMaster.SKM_Sausage` (`self.PlayerReference`)) (`/Game/Main/Core/DataAssets/PDA_ItemInfo.Socket` _output_get_2) "SnapToTarget" "SnapToTarget" "SnapToTarget" true))

(fn `DetachItem`
  (params (Item :type "/Game/Main/Core/Items/BP_ItemMaster Object Reference"))
  (bind _item (`local.Item`))
  (bind _staticmesh (`/Game/Main/Core/Items/BP_ItemMaster.StaticMesh` _item))
  (bind _capsule (`/Game/Main/Core/Player/BP_CharacterMaster.Capsule` (`self.PlayerReference`)))
  (`Actor.K2_DetachFromActor` Item "KeepWorld" "KeepWorld" "KeepWorld")
  (`PrimitiveComponent.SetCollisionEnabled` _staticmesh "QueryAndPhysics")
  (`PrimitiveComponent.SetCollisionEnabled` (`/Game/Main/Core/Items/BP_ItemMaster.Sphere` _item) "QueryOnly")
  (`PrimitiveComponent.SetSimulatePhysics` _staticmesh true)
  (`PrimitiveComponent.AddImpulse` _staticmesh (+ (`SceneComponent.K2_GetComponentLocation` _capsule) (* (`SceneComponent.GetUpVector` _capsule) 25000.0)) "None" false)
  (set `self.HeldItem` null)
  (return))