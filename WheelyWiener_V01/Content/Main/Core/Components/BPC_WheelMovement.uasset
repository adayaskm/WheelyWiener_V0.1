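; Movement component that drives a physics-simulated wheelchair pawn from forward and turn input values.
; On BeginPlay it caches its BP_WheelChairPawn owner.
; Each Tick it applies force along the pawn's forward vector and torque around its up vector to the wheelchair mesh, scaled by delta time.
; Linear and angular speed clamps exist in the graph but are disconnected, so neither limit takes effect.
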(event `self.ReceiveBeginPlay`
  (bind _asbp_wheel_chair_pawn (cast `/Game/Main/Core/Player/BP_WheelChairPawn` (`self.GetOwner`)))
  (set `self.OnwerPawn` _asbp_wheel_chair_pawn))

(event `self.ReceiveTick`
  (params (DeltaSeconds :type "Float (single-precision)"))
  (bind _onwerpawn (`self.OnwerPawn`))
  (bind _onwerpawn_2 (`self.OnwerPawn`))
  (`PrimitiveComponent.AddForce` (`/Game/Main/Core/Player/BP_WheelChairPawn.SMM_WheelChair` _onwerpawn_2) (* (`Actor.GetActorForwardVector` _onwerpawn_2) (* (`self.InputForward`) (`self.DriveForce`) DeltaSeconds)) "None" false)
  (`PrimitiveComponent.AddTorqueInRadians` (`/Game/Main/Core/Player/BP_WheelChairPawn.SMM_WheelChair` _onwerpawn) (* (`Actor.GetActorUpVector` _onwerpawn) (* (`self.InputRight`) (`self.TurnTorque`) DeltaSeconds)) "None" false))