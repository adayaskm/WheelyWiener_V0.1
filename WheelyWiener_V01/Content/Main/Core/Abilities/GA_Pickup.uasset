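; Gameplay ability that lets a character pick up, swap or drop items, running its logic only with authority.
; It reads the target item from the event data, rejecting it if already attached to an actor or not within a fixed distance.
; The character's interaction detector component detaches any held item before attaching the new one.
; Without a valid item target, it drops the held item instead.
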(event `self.K2_ActivateAbility`
  (`self.K2_HasAuthority`
    (:`True`
      (bind _asbp_character_master (cast `/Game/Main/Core/Player/BP_CharacterMaster` (`self.GetAvatarActorFromActorInfo` self))
        (:`then`
          (bind _asbp_item_master (cast `/Game/Main/Core/Items/BP_ItemMaster` (`.Target` (break `GameplayEventData` (`self.CurrentEventData`))))
            (:`then`
              (`/Engine/EditorBlueprintResources/StandardMacros.IsValid` (`Actor.GetAttachParentActor` _asbp_item_master)
                (:`Is Valid`
                  (`self.K2_EndAbility` self))
                (:`Is Not Valid`
                  (if (< (`KismetMathLibrary.VSize` (- (`Actor.K2_GetActorLocation` _asbp_item_master) (`Actor.K2_GetActorLocation` _asbp_character_master))) 2500.0)
                    (bind _bpc_interactiondetector (`/Game/Main/Core/Player/BP_CharacterMaster.BPC_InteractionDetector` _asbp_character_master))
                    (bind _helditem (`/Game/Main/Core/Components/BPC_InteractionDetector.HeldItem` _bpc_interactiondetector))
                    (`/Engine/EditorBlueprintResources/StandardMacros.IsValid` _helditem
                      (:`Is Valid`
                        (`/Game/Main/Core/Components/BPC_InteractionDetector.DetachItem` _bpc_interactiondetector _helditem)
                        (`/Game/Main/Core/Components/BPC_InteractionDetector.AttachItem` _bpc_interactiondetector _asbp_item_master)
                        (`self.K2_EndAbility` self))
                      (:`Is Not Valid`
                        (`/Game/Main/Core/Components/BPC_InteractionDetector.AttachItem` _bpc_interactiondetector _asbp_item_master)
                        (`self.K2_EndAbility` self)))
                    (else
                      (`self.K2_EndAbility` self))))))
            (:`CastFailed`
              (`/Engine/EditorBlueprintResources/StandardMacros.IsValid` _helditem
                (:`Is Valid`
                  (`/Game/Main/Core/Components/BPC_InteractionDetector.DetachItem` _bpc_interactiondetector _helditem)
                  (`self.K2_EndAbility` self))
                (:`Is Not Valid`
                  (`self.K2_EndAbility` self))))))
        (:`CastFailed`
          (`self.K2_EndAbility` self))))
    (:`False`
      (`self.K2_EndAbility` self))))