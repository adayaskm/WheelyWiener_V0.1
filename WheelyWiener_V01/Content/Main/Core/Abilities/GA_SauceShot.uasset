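; Gameplay ability that fires sauce-shot projectiles from the character's held item.
; On activation, it traces 2500 units along the player camera's forward vector, ignoring the character and held item.
; It spawns a BP_ProjectileMaster at every held-mesh socket, rotated toward the trace's end point rather than any impact point.
; CancelAbility is called inside the socket loop after each spawn, with no EndAbility call.
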(event `self.K2_ActivateAbility`
  (bind _asbp_character_master (cast `/Game/Main/Core/Player/BP_CharacterMaster` (`self.GetAvatarActorFromActorInfo`)))
  (bind _rootcomponent (`Actor.RootComponent` (`PlayerController.PlayerCameraManager` (`/Game/Main/Core/Player/BP_CharacterMaster.PlayerControllerReference` _asbp_character_master))))
  (bind _returnvalue (`SceneComponent.K2_GetComponentLocation` _rootcomponent))
  (bind _outhit (`KismetSystemLibrary.LineTraceSingle` _returnvalue (+ _returnvalue (* (`SceneComponent.GetForwardVector` _rootcomponent) 2500.0)) "TraceTypeQuery1" false (`|MakeArray` _asbp_character_master (`/Game/Main/Core/Components/BPC_InteractionDetector.HeldItem` (`/Game/Main/Core/Player/BP_CharacterMaster.BPC_InteractionDetector` _asbp_character_master)) :!type "Actor Object Reference")))
  (bind _staticmesh (`/Game/Main/Core/Items/BP_ItemMaster.StaticMesh` (`/Game/Main/Core/Components/BPC_InteractionDetector.HeldItem` (`/Game/Main/Core/Player/BP_CharacterMaster.BPC_InteractionDetector` _asbp_character_master))))
  (for _array_element (`SceneComponent.GetAllSocketNames` _staticmesh)
    (bind _returnvalue_location (`KismetMathLibrary.BreakTransform` (`SceneComponent.GetSocketTransform` _staticmesh _array_element "RTS_World")))
    (`|SpawnActorFromClass` "/Game/Main/Core/Items/BP_ProjectileMaster.BP_ProjectileMaster_C" (`KismetMathLibrary.MakeTransform` _returnvalue_location (`KismetMathLibrary.FindLookAtRotation` (`KismetMathLibrary.MakeVector` (.x _returnvalue_location) (.y _returnvalue_location) (.z _returnvalue_location)) (`.TraceEnd` (`GameplayStatics.BreakHitResult` _outhit)))) "AdjustIfPossibleButAlwaysSpawn" "MultiplyWithRoot" null null)
    (`self.K2_CancelAbility`)))