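; GA_Throw is a gameplay ability that throws the sauce item a character is holding toward the aimed point.
; Only the authority runs the throw, re-tracing along the aim ray from event target data and solving an arc velocity to the hit or range limit.
; It detaches the item, ignores collision with the thrower, applies the velocity a tick later, and records the thrown state and thrower.
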(event `self.K2_ActivateAbility`
  (bind (_bblockinghit _binitialoverlap _time _distance _location _impactpoint _normal _impactnormal _physmat _hitactor _hitcomponent _hitbonename _bonename _hititem _elementindex _faceindex _tracestart) (`GameplayStatics.BreakHitResult` (`AbilitySystemBlueprintLibrary.GetHitResultFromTargetData` (`.TargetData` (break `GameplayEventData` (`self.CurrentEventData`))))))
  (bind _returnvalue (+ _tracestart (* (`KismetMathLibrary.Normal` (- _location _tracestart)) 3000.0)))
  (`self.K2_HasAuthority`
    (:`True`
      (bind _asbp_character_master (cast `/Game/Main/Core/Player/BP_CharacterMaster` (`self.GetAvatarActorFromActorInfo`))
        (:`then`
          (bind _bpc_interactiondetector (`/Game/Main/Core/Player/BP_CharacterMaster.BPC_InteractionDetector` _asbp_character_master))
          (bind _asbp_sauce_master (cast `/Game/Main/Core/Items/BP_SauceMaster` (`/Game/Main/Core/Components/BPC_InteractionDetector.HeldItem` _bpc_interactiondetector))
            (:`then`
              (set `self.As BP Character Master` _asbp_character_master)
              (bind (_outhit _returnvalue_2) (`KismetSystemLibrary.LineTraceSingle` _tracestart _returnvalue "TraceTypeQuery1"))
              (bind _staticmesh (`/Game/Main/Core/Items/BP_ItemMaster.StaticMesh` _asbp_sauce_master))
              (bind _outlaunchvelocity (`GameplayStatics.SuggestProjectileVelocity_CustomArc` (`SceneComponent.K2_GetComponentLocation` _staticmesh) (select `bool` _returnvalue_2 :`false` _returnvalue :`true` (`.Location` (`GameplayStatics.BreakHitResult` _outhit))) -1500.0 0.35))
              (`/Game/Main/Core/Components/BPC_InteractionDetector.DetachItem` _bpc_interactiondetector _asbp_sauce_master)
              (`PrimitiveComponent.IgnoreActorWhenMoving` _staticmesh _asbp_character_master true)
              (`KismetSystemLibrary.DelayUntilNextTick`)
              (`PrimitiveComponent.SetPhysicsLinearVelocity` _staticmesh _outlaunchvelocity false "None")
              (set `/Game/Main/Core/Items/BP_SauceMaster.bIsThrown` true _asbp_sauce_master)
              (set `/Game/Main/Core/Items/BP_SauceMaster.ThrowerReference` _asbp_character_master _asbp_sauce_master)
              (`self.K2_EndAbility`))
            (:`CastFailed`
              (`self.K2_EndAbility`))))
        (:`CastFailed`
          (`self.K2_EndAbility`))))
    (:`False`
      (`self.K2_EndAbilityLocally`))))