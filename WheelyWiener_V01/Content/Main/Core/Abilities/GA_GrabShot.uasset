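; Gameplay ability that lets a character grab physics objects with the grab pistol.
; On activation it runs TryGrab and ends; the locally controlled player, holding left mouse, line-traces from the eyes for BPI_Grab actors.
; ResolveGrabComponent picks the simulating hit component or falls back to a static mesh, which the character's PhysicsHandle grabs, storing a minimum-clamped distance on the pistol.
; CheckBelow, a debug-drawn vertical trace helper, is not called here.
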(event `self.K2_ActivateAbility`
  (`self.TryGrab`)
  (`self.K2_EndAbility`))

(fn `ResolveGrabComponent`
  (params (HitActor :type "Actor Object Reference") (HitComponent :type "PrimitiveComponent Object Reference"))
  (returns (GrabComponent :type "PrimitiveComponent Object Reference"))
  (return (select `bool` (`SceneComponent.IsSimulatingPhysics` HitComponent "None") :`false` (`Actor.GetComponentByClass` HitActor "/Script/Engine.StaticMeshComponent") :`true` HitComponent :!type "PrimitiveComponent Object Reference")))

(fn `TryGrab`
  (locals (IgnoreActors :type "Array of Actor Object Reference"))
  (bind _as_bp_character_master (`self.As BP Character Master`))
  (bind _ignoreactors (`local.IgnoreActors`))
  (bind (_outlocation _outrotation) (`Actor.GetActorEyesViewPoint` _as_bp_character_master))
  (bind _asbp_character_master (cast `/Game/Main/Core/Player/BP_CharacterMaster` (`self.GetAvatarActorFromActorInfo`)))
  (bind _output_get (set `self.As BP Character Master` _asbp_character_master))
  (`self.IsLocallyControlled`
    (:`True`
      (if (`/Game/Main/Core/Player/BP_CharacterMaster.bGrabbing` _output_get)
        _
        (elif (not (not (`PlayerController.IsInputKeyDown` (`/Game/Main/Core/Player/BP_CharacterMaster.PlayerControllerReference` (`self.As BP Character Master`)) "LeftMouseButton")))
          (bind _helditem (`/Game/Main/Core/Components/BPC_InteractionDetector.HeldItem` (`/Game/Main/Core/Player/BP_CharacterMaster.BPC_InteractionDetector` _output_get)))
          (bind _asbp_grab_pistol (cast `/Game/Main/Core/Items/BP_GrabPistol` _helditem))
          (`KismetArrayLibrary.Array_Add` _ignoreactors _as_bp_character_master)
          (`KismetArrayLibrary.Array_Add` _ignoreactors _helditem)
          (bind (_outhit _returnvalue) (`KismetSystemLibrary.LineTraceSingle` _outlocation (+ _outlocation (* (`KismetMathLibrary.GetForwardVector` _outrotation) (`/Game/Main/Core/Items/BP_GrabPistol.GrabRange` _asbp_grab_pistol))) "TraceTypeQuery1" false (`local.IgnoreActors`)))
          (if (not (not _returnvalue))
            (bind (_bblockinghit _binitialoverlap _time _distance _location _impactpoint _normal _impactnormal _physmat _hitactor _hitcomponent) (`GameplayStatics.BreakHitResult` _outhit))
            (if (not (not (`KismetSystemLibrary.DoesImplementInterface` _hitactor "/Game/Main/Core/Interfaces/BPI_Grab.BPI_Grab_C")))
              (bind _grabcomponent (`self.ResolveGrabComponent` _hitactor _hitcomponent))
              (if (not (not (`SceneComponent.IsSimulatingPhysics` _grabcomponent "None")))
                (`PhysicsHandleComponent.GrabComponentAtLocationWithRotation` (`/Game/Main/Core/Player/BP_CharacterMaster.PhysicsHandle` _output_get) _grabcomponent "None" _impactpoint (`SceneComponent.K2_GetComponentRotation` _grabcomponent))
                (bind _mingrabdistance (`/Game/Main/Core/Items/BP_GrabPistol.MinGrabDistance` _asbp_grab_pistol))
                (set `/Game/Main/Core/Items/BP_GrabPistol.GrabDistance` (select `bool` (> _distance _mingrabdistance) :`false` _mingrabdistance :`true` _distance :!type "Float (single-precision)") _asbp_grab_pistol)
                (set `/Game/Main/Core/Player/BP_CharacterMaster.bGrabbing` true _output_get)))))))))