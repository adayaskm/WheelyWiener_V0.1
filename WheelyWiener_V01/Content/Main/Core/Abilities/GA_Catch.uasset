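; Gameplay ability that makes the avatar character catch a sauce item and hold it.
; It reads the sauce from the triggering event data's optional object and uses the character's interaction detector component to detach any held item, then attach the sauce.
; The ability is instantaneous, ending right after the swap.
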(event `self.K2_ActivateAbility`
  (bind _asbp_sauce_master (cast `/Game/Main/Core/Items/BP_SauceMaster` (`.OptionalObject` (break `GameplayEventData` (`self.CurrentEventData`))))
    (:`then`
      (bind _asbp_character_master (cast `/Game/Main/Core/Player/BP_CharacterMaster` (`self.GetAvatarActorFromActorInfo` self))
        (:`then`
          (bind _bpc_interactiondetector (`/Game/Main/Core/Player/BP_CharacterMaster.BPC_InteractionDetector` _asbp_character_master))
          (bind _helditem (`/Game/Main/Core/Components/BPC_InteractionDetector.HeldItem` _bpc_interactiondetector))
          (if (!= _helditem null)
            (`/Game/Main/Core/Components/BPC_InteractionDetector.DetachItem` _bpc_interactiondetector _helditem))
          (`/Game/Main/Core/Components/BPC_InteractionDetector.AttachItem` _bpc_interactiondetector _asbp_sauce_master))
        (:`CastFailed`
          _)))
    (:`CastFailed`
      _))
  (`self.K2_EndAbility` self))