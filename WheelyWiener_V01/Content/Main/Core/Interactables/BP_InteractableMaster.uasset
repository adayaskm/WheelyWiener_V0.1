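; Base interactable actor that shows and hides an interact prompt widget around its WidgetRadius overlap volume.
; Begin overlap toggles the prompt when the other actor has a BPC_InteractionDetector component, while end overlap toggles it for any actor.
; Visibility alternates through a FlipFlop rather than being set explicitly.
; The construction script places the widget at the top of the radius bounds.
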(event `TogglePromptVisibility`
  (bind _widget (`self.Widget`))
  ; Toggle Interact Widget
  (`/Engine/EditorBlueprintResources/StandardMacros.FlipFlop`
    (:`A`
      (`SceneComponent.SetVisibility` _widget true false))
    (:`B`
      (`SceneComponent.SetVisibility` _widget false false))))

(event `self.WidgetRadius.OnComponentBeginOverlap`
  (params (OverlappedComponent :type "PrimitiveComponent Object Reference") (OtherActor :type "Actor Object Reference") (OtherComp :type "PrimitiveComponent Object Reference") (OtherBodyIndex :type Integer) (bFromSweep :type Boolean) (SweepResult :type "HitResult Structure (by ref)"))
  ; Toggle Interact Widget
  (`/Engine/EditorBlueprintResources/StandardMacros.IsValid` (`self.GetComponentByClass` OtherActor "/Game/Main/Core/Components/BPC_InteractionDetector.BPC_InteractionDetector_C")
    (:`Is Valid`
      (`self.TogglePromptVisibility`))))

(event `self.WidgetRadius.OnComponentEndOverlap`
  (params (OverlappedComponent :type "PrimitiveComponent Object Reference") (OtherActor :type "Actor Object Reference") (OtherComp :type "PrimitiveComponent Object Reference") (OtherBodyIndex :type Integer))
  ; Toggle Interact Widget
  (`self.TogglePromptVisibility`))

(fn `UserConstructionScript`
  (bind (_origin _boxextent _sphereradius) (`KismetSystemLibrary.GetComponentBounds` (`self.WidgetRadius`)))
  (`SceneComponent.K2_SetWorldLocation` (`self.Widget`) (`KismetMathLibrary.MakeVector` (.x _origin) (.y _origin) (+ (.z _origin) _sphereradius)) false false))