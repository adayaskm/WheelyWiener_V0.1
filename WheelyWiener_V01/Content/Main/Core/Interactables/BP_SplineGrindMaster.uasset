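; Spline-based actor, named as a master for grind rails, that builds a collidable mesh track along its spline.
; The construction script splits the spline by a set segment distance and adds a spline mesh per segment, clamping tangents to that distance.
; Each segment gets the configured mesh, material and forward axis, uses a custom collision object type, and overlaps pawns and physics bodies.
; The event graph holds no gameplay logic.
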(event `self.ReceiveTick`
  (params (DeltaSeconds :type "Float (single-precision)"))
  (`parent.ReceiveTick` DeltaSeconds))

(fn `UserConstructionScript`
  (bind _spline (`self.Spline`))
  (for _index (range (+ (`KismetMathLibrary.FTrunc` (/ (`SplineComponent.GetSplineLength` _spline) (`self.Distance`))) 1))
    (bind _returnvalue (`AddComponent|NODE_AddSplineMeshComponent-0`))
    (`SplineMeshComponent.SetForwardAxis` _returnvalue (`self.In Forward Axis`) true)
    (`StaticMeshComponent.SetStaticMesh` _returnvalue (`self.Mesh`))
    (`PrimitiveComponent.SetMaterial` _returnvalue 0 (`self.Material`))
    (bind _returnvalue_2 (* _index (`self.Distance`)))
    (bind _returnvalue_3 (* (+ _index 1) (`self.Distance`)))
    (`SplineMeshComponent.SetStartAndEnd` _returnvalue (`SplineComponent.GetLocationAtDistanceAlongSpline` _spline _returnvalue_2 "Local") (`KismetMathLibrary.ClampVectorSize` (`SplineComponent.GetTangentAtDistanceAlongSpline` _spline _returnvalue_2 "Local") 0.0 (`self.Distance`)) (`SplineComponent.GetLocationAtDistanceAlongSpline` _spline _returnvalue_3 "Local") (`KismetMathLibrary.ClampVectorSize` (`SplineComponent.GetTangentAtDistanceAlongSpline` _spline _returnvalue_3 "Local") 0.0 (`self.Distance`)) true)
    (`PrimitiveComponent.SetCollisionEnabled` _returnvalue "QueryAndPhysics")
    (`PrimitiveComponent.SetCollisionObjectType` _returnvalue "ECC_GameTraceChannel1")
    (`PrimitiveComponent.SetCollisionResponseToChannel` _returnvalue "ECC_Pawn" "ECR_Overlap")
    (`PrimitiveComponent.SetCollisionResponseToChannel` _returnvalue "ECC_PhysicsBody" "ECR_Overlap")))